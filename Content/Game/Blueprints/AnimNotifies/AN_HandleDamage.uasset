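; AN_HandleDamage is an animation notify that triggers a character's attack handling from a point in an animation.
; When it fires, it casts the mesh owner to BP_Character and calls HandleAttack with its SocketName, returning whether that cast succeeded.
; Its displayed notify name includes the socket name.
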(fn `GetNotifyName`
  (returns (ReturnValue :type String))
  (return (`KismetStringLibrary.Concat_StrStr` "Handle Damage: " (`KismetStringLibrary.Conv_NameToString` (`self.SocketName`)))))

(fn `Received_Notify`
  (params (MeshComp :type "SkeletalMeshComponent Object Reference") (Animation :type "AnimSequenceBase Object Reference"))
  (returns (ReturnValue :type Boolean))
  (bind _returnvalue (`ActorComponent.GetOwner` MeshComp))
  (`/Engine/EditorBlueprintResources/StandardMacros.IsValid` _returnvalue
    (:`Is Valid`
      (bind _asbp_character (cast `/Game/Game/Blueprints/BP_Character` _returnvalue)
        (:`then`
          (`/Game/Game/Blueprints/BP_Character.HandleAttack` _asbp_character (`self.SocketName`))
          (return true))
        (:`CastFailed`
          (return false))))
    (:`Is Not Valid`
      (return false))))